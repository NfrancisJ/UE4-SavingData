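; BP_PlayerCharacter is the player character Blueprint, handling basic movement and look input.
; Move and strafe axes add movement along the control rotation's forward and right vectors, while look axes feed controller pitch and yaw.
; Pressing P fires the save, load and reset dispatchers in immediate succession on the SaveGameObject held by BP_GameInstance.
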(event `InputAxis|Move`
  (params (AxisValue :type "Float (single-precision)"))
  ;[0 0 0] Charater Movement
  (`self.AddMovementInput` (`KismetMathLibrary.GetForwardVector` (`self.GetControlRotation`)) AxisValue))

(event `InputAxis|Straf`
  (params (AxisValue :type "Float (single-precision)"))
  ;[0 0 0] Charater Movement
  (`self.AddMovementInput` (`KismetMathLibrary.GetRightVector` (`self.GetControlRotation`)) AxisValue))

(event `InputAxis|Look-Y`
  (params (AxisValue :type "Float (single-precision)"))
  ;[0 0 0] Charater Movement
  (`self.AddControllerPitchInput` AxisValue))

(event `InputAxis|Look-X`
  (params (AxisValue :type "Float (single-precision)"))
  ;[0 0 0] Charater Movement
  (`self.AddControllerYawInput` AxisValue))

(event `Key|P`
  (params (Key :type "Key Structure"))
  (:`Pressed`
    (bind _asbp_game_instance (cast `/Game/MyGame/Blueprints/Core/BP_GameInstance` (`GameplayStatics.GetGameInstance`)))
    (bind _savegameobject (`/Game/MyGame/Blueprints/Core/BP_GameInstance.SaveGameObject` _asbp_game_instance))
    (`/Game/MyGame/Blueprints/Core/BP_SaveGame.OnSave` _savegameobject)
    (`/Game/MyGame/Blueprints/Core/BP_SaveGame.OnLoad` _savegameobject)
    (`/Game/MyGame/Blueprints/Core/BP_SaveGame.OnReset` _savegameobject)))

(fn `UserConstructionScript`)
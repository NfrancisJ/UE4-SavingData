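; BP_ActorSave_BASE is a base actor for objects that save, load and reset their data through BP_GameInstance events.
; On BeginPlay it caches the game instance and binds its OnSave and OnLoad dispatchers to handlers that call SaveData and LoadData.
; OnReset is unbound rather than bound there, so that dispatcher is not hooked to ResetData.
; SaveData, LoadData and ResetData are empty, apparently left for child Blueprints to override.
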(event `self.ReceiveBeginPlay`
  (bind _asbp_game_instance (cast `/Game/MyGame/Blueprints/Core/BP_GameInstance` (`GameplayStatics.GetGameInstance`)))
  (bind _output_get (set `self.GameInstanceRef` _asbp_game_instance))
  ;[0 0 0] Install Save/Load/Reset Events
  (add `/Game/MyGame/Blueprints/Core/BP_GameInstance.OnSave` _output_get (delegate `OnSave_Event`))
  (add `/Game/MyGame/Blueprints/Core/BP_GameInstance.OnLoad` _output_get (delegate `OnLoad_Event`))
  (remove `/Game/MyGame/Blueprints/Core/BP_GameInstance.OnReset` _output_get (delegate `OnReset_Event`)))

(event `OnSave_Event`
  ;[0 0 0] Install Save/Load/Reset Events
  (`self.SaveData`))

(event `OnLoad_Event`
  ;[0 0 0] Install Save/Load/Reset Events
  (`self.LoadData`))

(event `OnReset_Event`
  ;[0 0 0] Install Save/Load/Reset Events
  (`self.ResetData`))

(fn `LoadData`)

(fn `ResetData`)

(fn `SaveData`)

(fn `UserConstructionScript`)
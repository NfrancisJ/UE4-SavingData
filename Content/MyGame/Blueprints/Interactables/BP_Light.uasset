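; BP_Light is an interactable light that toggles its point light whenever an actor begins overlapping it and remembers that state.
; On BeginPlay it casts to BP_GameInstance and sets visibility from the save object's SLight map, keyed by the actor's object name.
; Each toggle adds the entry when lit or removes it when off, updating the map without writing the save to disk here.
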(event `self.ReceiveBeginPlay`
  (bind _asbp_game_instance (cast `/Game/MyGame/Blueprints/Core/BP_GameInstance` (`GameplayStatics.GetGameInstance`)))
  (set `self.GameInstanceRef` _asbp_game_instance)
  ;[0 0 0] When loaded, check the MAP for what its state should be.
  (`SceneComponent.SetVisibility` (`self.PointLight`) (break `/Game/MyGame/Blueprints/Core/Structs/SLight` (`BlueprintMapLibrary.Map_Find` (`/Game/MyGame/Blueprints/Core/BP_SaveGame.SLight` (`/Game/MyGame/Blueprints/Core/BP_GameInstance.SaveGameObject` (`self.GameInstanceRef`))) (`KismetSystemLibrary.GetObjectName` self))) false))

(event `self.ReceiveActorBeginOverlap`
  (params (OtherActor :type "Actor Object Reference"))
  (bind _returnvalue (`KismetSystemLibrary.GetObjectName` self))
  (bind _slight (`/Game/MyGame/Blueprints/Core/BP_SaveGame.SLight` (`/Game/MyGame/Blueprints/Core/BP_GameInstance.SaveGameObject` (`self.GameInstanceRef`))))
  (`SceneComponent.ToggleVisibility` (`self.PointLight`) false)
  ;[0 0 0] If the light has changed from OFF to ON, save it to the MAP, else remove it.
  (if (`SceneComponent.bVisible` (`self.PointLight`))
    (`BlueprintMapLibrary.Map_Add` _slight _returnvalue (make `/Game/MyGame/Blueprints/Core/Structs/SLight` true))
    (else
      (`BlueprintMapLibrary.Map_Remove` _slight _returnvalue))))

(fn `UserConstructionScript`)